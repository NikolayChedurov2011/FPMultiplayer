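; BP_AmmoWeapon is a weapon Blueprint that adds ammunition and magazine logic to its parent's Fire and Reload behavior.
; It tracks one total ammo count, clamped on pickup, and derives loaded rounds via modulo of magazine size, with a Reloaded flag marking a full magazine.
; Fire, and Reload after a retriggerable delay, recount the magazine and broadcast it.
; Helper functions check ammo state and scale fire animation play rate to shots per second.
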(event `self.ReceiveBeginPlay`
  (`parent.ReceiveBeginPlay`))

(event `self.Fire`
  (`parent.Fire`)
  (`self.CounAmmoInMagazine`))

(event `self.Reload`
  (`parent.Reload`)
  (`KismetSystemLibrary.RetriggerableDelay` (`self.ReloadTime`))
  (`self.CounAmmoInMagazine`))

(fn `ApplyAmmo`
  (params (Ammo :type Integer))
  (bind _output_get (set `self.CurrentAmmo` (`KismetMathLibrary.Min` (+ Ammo (`self.CurrentAmmo`)) (`self.MaxAmmo`))))
  (`self.OnAmmoChanged` _output_get))

(fn `CheckAmmunition`
  (returns (bAmmunition :type Boolean))
  (return (> (`self.CurrentAmmo`) 0)))

(fn `CheckLoaded`
  (returns (bLoaded :type Boolean))
  (return (not (and (== (mod (`self.CurrentAmmo`) (`self.AmmoPerMagazine`)) 0) (not (`self.bReloaded`))))))

(fn `CounAmmoInMagazine`
  (if (`self.bReloaded`)
    (set `self.LoadedAmmo` (`self.AmmoPerMagazine`))
    (else
      (set `self.LoadedAmmo` (mod (`self.CurrentAmmo`) (`self.AmmoPerMagazine`)))))
  (`self.OnLoadedAmmo` (`self.LoadedAmmo`)))

(fn `GetFireAnimationPlayRate`
  (returns (PlayRate :type "Float (double-precision)"))
  (return (* (`AnimSequenceBase.SequenceLength` (`self.W_Fire`)) (`self.ShotsPerSecond`))))

(fn `IsFullAmmo`
  (returns (bIsFull :type Boolean))
  (return (== (`self.CurrentAmmo`) (`self.MaxAmmo`))))

(fn `UseAmmunition`
  (bind _result (`/Engine/EditorBlueprintResources/StandardMacros.DecrementInt` (`self.CurrentAmmo`))
    (:`  `
      (`self.OnAmmoChanged` _result))))

(fn `UserConstructionScript`
  (`parent.UserConstructionScript`))