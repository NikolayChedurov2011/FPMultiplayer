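; Base projectile actor for multiplayer projectile weapons, driven by a collision box and projectile movement.
; A box hit on anything other than its owner or instigator triggers OnHit, which waits a configurable delay.
; It then spawns a damage actor of a configurable class at its location, passing on the owner, and destroys itself.
; The explosion effect event only destroys the actor, and the bounce event is empty.
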(event `self.Box.OnComponentHit`
  (params (HitComponent :type "PrimitiveComponent Object Reference") (OtherActor :type "Actor Object Reference") (OtherComp :type "PrimitiveComponent Object Reference") (NormalImpulse :type "Vector Structure") (Hit :type "HitResult Structure (by ref)"))
  (if (and (!= OtherActor (`self.GetOwner`)) (!= OtherActor (`self.GetInstigator`)))
    (`self.OnHit`)))

(event `OnHit`
  (`KismetSystemLibrary.Delay` (`self.HitDestroyDelay`))
  (`|SpawnActorFromClass` (`self.DamageActorClass`) (`KismetMathLibrary.MakeTransform` (`self.K2_GetActorLocation`)) "Undefined" "OverrideRootScale" (`self.GetOwner`) null)
  (`self.SpawnExplosionEffectAndDestroy`))

(event `SpawnExplosionEffectAndDestroy`
  (`self.K2_DestroyActor`))

(event `self.ProjectileMovement.OnProjectileBounce`
  (params (ImpactResult :type "HitResult Structure (by ref)") (ImpactVelocity :type "Vector Structure (by ref)")))

(fn `UserConstructionScript`)