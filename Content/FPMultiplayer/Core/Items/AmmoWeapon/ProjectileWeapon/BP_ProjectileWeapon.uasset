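; BP_ProjectileWeapon is a weapon Blueprint that fires by spawning projectile actors.
; On fire, it runs the parent logic, then spawns its ProjectileClass at the skeletal mesh's Muzzle socket.
; The projectile faces along the owner's actor rotation rather than the socket's and takes its scale from the projectile class defaults.
; The weapon is set as the projectile's owner and the owning pawn as its instigator.
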(event `self.OnFired`
  (`parent.OnFired`)
  (`|SpawnActorFromClass` (`self.ProjectileClass`) (`KismetMathLibrary.MakeTransform` (`SceneComponent.GetSocketLocation` (`self.SkeletalMesh`) "Muzzle") (`self.K2_GetActorRotation` (`self.GetOwner`)) (`.ProjectileScale` (defaults `Object` (`self.ProjectileClass`)))) "Undefined" "OverrideRootScale" self (cast `Pawn` (`self.GetOwner`) :!pure true)))

(fn `UserConstructionScript`
  (`parent.UserConstructionScript`))