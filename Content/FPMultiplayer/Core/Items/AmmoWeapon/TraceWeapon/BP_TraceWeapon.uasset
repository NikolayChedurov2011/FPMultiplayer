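; BP_TraceWeapon is a hitscan-style ammo weapon that fires a line trace from the muzzle socket along the owner's forward vector.
; On a hit, it spawns a BP_TracerActor set to travel at TraceSpeed and expire on reaching the impact point.
; After a matching travel-time delay, it spawns the DamageActorClass actor at the hit location, simulating bullet flight time.
; Misses spawn nothing, and the trace draws debug lines.
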(event `self.OnFired`
  (bind _tracespeed (`self.TraceSpeed`))
  (bind _returnvalue (`SceneComponent.GetSocketLocation` (`self.SkeletalMesh`) "Muzzle"))
  (`parent.OnFired`)
  (bind (_outhit _returnvalue_2) (`KismetSystemLibrary.LineTraceSingle` _returnvalue (+ _returnvalue (* (`self.GetActorForwardVector` (`self.GetOwner`)) (`self.TraceDistance`))) "TraceTypeQuery2" false (`|MakeArray` (`self.GetOwner`)) "ForDuration" true (struct :`R` 1.0 :`A` 1.0) (struct :`G` 1.0 :`A` 1.0) 30.0))
  (if _returnvalue_2
    (bind _returnvalue_3 (`|SpawnActorFromClass` "/Game/FPMultiplayer/Core/Items/AmmoWeapon/TraceWeapon/BP_TracerActor.BP_TracerActor_C" (`KismetMathLibrary.MakeTransform` _returnvalue (`self.K2_GetActorRotation` (`self.GetOwner`))) "Undefined" "OverrideRootScale" self null))
    (bind _returnvalue_4 (/ (`.Distance` (`GameplayStatics.BreakHitResult` _outhit)) _tracespeed))
    (`/Game/FPMultiplayer/Core/Items/AmmoWeapon/TraceWeapon/BP_TracerActor.SetParams` _returnvalue_3 _tracespeed _returnvalue_4 null)
    (`KismetSystemLibrary.Delay` _returnvalue_4)
    (`|SpawnActorFromClass` (`self.DamageActorClass`) (`KismetMathLibrary.MakeTransform` (`.Location` (`GameplayStatics.BreakHitResult` _outhit))) "Undefined" "OverrideRootScale" self null)))

(fn `UserConstructionScript`
  (`parent.UserConstructionScript`))