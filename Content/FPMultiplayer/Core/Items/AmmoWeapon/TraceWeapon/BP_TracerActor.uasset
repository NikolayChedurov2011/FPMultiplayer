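; BP_TracerActor is a short-lived tracer visual actor, likely for trace weapons.
; SetParams stores the speed, assigns the particle template, sets that component hidden in game and sets the actor's lifespan.
; Once initialized, Tick moves it without sweeping, adding speed times delta time to the forward vector rather than scaling that vector.
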(event `SetParams`
  (params (TracerSpeed :type "Float (double-precision)") (DestroyTime :type "Float (double-precision)") (ParticleSystem :type "ParticleSystem Object Reference"))
  (bind _particlesystem (`self.ParticleSystem`))
  (set `self.TracerSpeed` TracerSpeed)
  (set `self.DestroyTime` DestroyTime)
  (`ParticleSystemComponent.SetTemplate` _particlesystem ParticleSystem)
  (`SceneComponent.SetHiddenInGame` _particlesystem true false)
  (set `self.bParamsSet` true)
  (`self.SetLifeSpan` (`self.DestroyTime`)))

(event `self.ReceiveTick`
  (params (DeltaSeconds :type "Float (single-precision)"))
  (if (`self.bParamsSet`)
    (`self.K2_AddActorWorldOffset` (+ (`self.GetActorForwardVector`) (* DeltaSeconds (`self.TracerSpeed`))))))

(fn `UserConstructionScript`)