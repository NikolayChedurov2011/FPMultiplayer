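; Base weapon Blueprint that defines the shared fire and reload flow, leaving ammo checks, ammo use, magazine counting and shot effects as stubs.
; Fire gates on readiness and ammo, then either consumes ammo and plays the fire montage, starts a reload, or calls NoAmmo.
; Montage play rate comes from an overridable function, and a notify is meant to trigger OnFired.
; Reload broadcasts its duration and blocks firing through a retriggerable delay.
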(event `self.ReceiveBeginPlay`
  (`self.CounAmmoInMagazine`))

(event `Fire`
  ;[1 1 1] Проверяем готовы ли мы стрелять, патроны, нужно ли перезарядиться. Если всё готово, то используем поеприпасы и вызываем следующее событие
  (if (`self.bReadyToFire`)
    (bind _bammunition (`self.CheckAmmunition`))
    (if _bammunition
      (bind _bloaded (`self.CheckLoaded`))
      (if _bloaded
        (set `self.bReadyToFire` false)
        (`self.UseAmmunition`)
        (set `self.bReloaded` false)
        (`self.OnReadyToFire`)
        (else
          (`self.Reload`)))
      (else
        (`self.NoAmmo`)))))

(event `OnReadyToFire`
  ;[1 1 1] Проигрываем монтаж стрельбы со скоростью, которая зависит отвыстрелов оружия в секунду, затем, в монтаже срабатывает нотифай, вызывающийсобытие OnFired
  (`|PlayMontage` (`self.SkeletalMesh`) (`self.W_Fire`) (`self.GetFireAnimationPlayRate`)
    (:`OnCompleted`
      _)
    (:`OnInterrupted`
      _))
  (set `self.bReadyToFire` true))

(event `Reload`
  (bind _reloadtime (`self.ReloadTime`))
  (set `self.bReloadInProgress` true)
  (set `self.bReadyToFire` false)
  (set `self.bInUse` true)
  (`self.OnReload` _reloadtime)
  (`KismetSystemLibrary.RetriggerableDelay` _reloadtime)
  (set `self.bReloadInProgress` false)
  (set `self.bReadyToFire` true)
  (set `self.bReloaded` true)
  (set `self.bInUse` false))

(event `OnFired`)

(event `NoAmmo`)

(event `OnEquipped`)

(event `OnUnequipped`)

(fn `CheckAmmunition`
  (returns (bAmmunition :type Boolean))
  (return false))

(fn `CheckLoaded`
  (returns (bLoaded :type Boolean))
  (return false))

(fn `CounAmmoInMagazine`)

(fn `GetFireAnimationPlayRate`
  (returns (PlayRate :type "Float (double-precision)"))
  (return 1.0))

(fn `UseAmmunition`)

(fn `UserConstructionScript`)