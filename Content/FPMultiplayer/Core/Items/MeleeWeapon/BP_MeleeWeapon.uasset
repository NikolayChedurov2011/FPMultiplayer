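; BP_MeleeWeapon is a melee weapon that deals point damage to what it strikes.
; Fire runs the parent logic and, on success, applies damage using the hit from GetOverlapInfo, crediting the instigator's controller.
; GetOverlapInfo sphere-traces from the humanoid pawn's camera along the owner's forward vector over the attack radius, with debug drawing left on.
; Use is allowed whenever UseFreezed is false.
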(fn `AbleToUse`
  (returns (Able :type Boolean))
  (return (not (`self.bUseFreezed`))))

(fn `Fire`
  (returns (Used :type Boolean))
  (bind _used (`parent.Fire`))
  (if _used
    (bind _hitresult (`self.GetOverlapInfo`))
    (bind (_bblockinghit _binitialoverlap _time _distance _location _impactpoint _normal _impactnormal _physmat _hitactor _hitcomponent _hitbonename _hititem _elementindex _faceindex _tracestart _traceend) (`GameplayStatics.BreakHitResult` _hitresult))
    (`GameplayStatics.ApplyPointDamage` _hitactor (`self.Damage`) (`KismetMathLibrary.GetDirectionUnitVector` _traceend _tracestart) _hitresult (`self.GetInstigatorController`) self)
    (return _used)
    (else
      (return false))))

(fn `GetOverlapInfo`
  (returns (HitResult :type "HitResult Structure"))
  (bind _asbp_humanoid_pawn (cast `/Game/FPMultiplayer/Core/Characters/BasePawn/BP_HumanoidPawn` (`self.GetInstigator`))
    (:`then`
      (bind _returnvalue (`SceneComponent.K2_GetComponentLocation` (`/Game/FPMultiplayer/Core/Characters/BasePawn/BP_HumanoidPawn.Camera` _asbp_humanoid_pawn)))
      (bind _outhit (`KismetSystemLibrary.SphereTraceSingleForObjects` _returnvalue (+ _returnvalue (* (`self.GetActorForwardVector` (`self.GetOwner`)) (`self.AttackRadius`))) (`self.SphereRadius`) (`|MakeArray` "ObjectTypeQuery1" "ObjectTypeQuery2" "ObjectTypeQuery3" :!type "EObjectTypeQuery Enum") false (`|MakeArray` (`self.GetInstigator`) self :!type "Actor Object Reference") "ForDuration"))
      (return _outhit))
    (:`CastFailed`
      (return))))

(fn `UserConstructionScript`
  (`parent.UserConstructionScript`))