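; BP_RechargablePickUp is a pickup that becomes available again after a recharge delay.
; On player overlap, a Recharge flag gates the impact, which calls the parent's logic, then stays false for RechargeDuration.
; When the delay ends, it unhides the particle system and repeats the impact and recharge cycle while the Pawn reference remains valid.
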(event `RechargedCosmetic`
  (`SceneComponent.SetHiddenInGame` (`self.ParticleSystem`) false true))

(event `self.OnPlayerBeginOverlap`
  (params (Player :type "Pawn Object Reference"))
  (bind _bready (`self.ReadyToImpact` Player))
  (if _bready
    (`self.PlayerImpact` Player :!label _label)
    (set `self.bRecharge` false)
    (`KismetSystemLibrary.Delay` (`self.RechargeDuration`))
    (set `self.bRecharge` true)
    (`self.RechargedCosmetic`)
    (if (`KismetSystemLibrary.IsValid` (`self.Pawn`))
      (goto _label))))

(event `self.OnPlayerEndOverlap`
  (params (Player :type "Pawn Object Reference")))

(event `self.PlayerImpact`
  (params (Player :type "Pawn Object Reference"))
  (`parent.PlayerImpact` Player))

(fn `ReadyToImpact`
  (params (Player :type "Pawn Object Reference"))
  (returns (bReady :type Boolean))
  (return (`self.bRecharge`)))

(fn `UserConstructionScript`
  (`parent.UserConstructionScript`))