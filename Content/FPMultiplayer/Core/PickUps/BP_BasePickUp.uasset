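; Base pickup actor for the FPMultiplayer game, with overridable hooks that react when a player touches its box trigger.
; Box overlap accepts actors implementing BPI_Health, caches their pawn and forwards it to the player overlap event.
; If ReadyToImpact passes (always true here), PlayerImpact runs ImpactCosmetic to hide the mesh, then the actor destroys itself.
; Leaving the box clears the cached pawn and fires an empty end-overlap hook.
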(event `ImpactCosmetic`
  (params (Player :type "Pawn Object Reference"))
  (`SceneComponent.SetHiddenInGame` (`self.StaticMesh`) true true))

(event `PlayerImpact`
  (params (Player :type "Pawn Object Reference"))
  (`self.ImpactCosmetic` Player))

(event `OnPlayerBeginOverlap`
  (params (Player :type "Pawn Object Reference"))
  (bind _bready (`self.ReadyToImpact` Player))
  (if _bready
    (`self.PlayerImpact` Player)
    (`self.K2_DestroyActor`)))

(event `OnPlayerEndOverlap`
  (params (Player :type "Pawn Object Reference")))

(event `self.Box.OnComponentBeginOverlap`
  (params (OverlappedComponent :type "PrimitiveComponent Object Reference") (OtherActor :type "Actor Object Reference") (OtherComp :type "PrimitiveComponent Object Reference") (OtherBodyIndex :type Integer) (bFromSweep :type Boolean) (SweepResult :type "HitResult Structure (by ref)"))
  (if (`KismetSystemLibrary.DoesImplementInterface` OtherActor "/Game/FPMultiplayer/Core/Interfaces/BPI_Health.BPI_Health_C")
    (bind _pawn (message `/Game/FPMultiplayer/Core/Interfaces/BPI_GetPawn.GetPawn` OtherActor))
    (bind _output_get (set `self.Pawn` _pawn))
    (`self.OnPlayerBeginOverlap` _output_get)))

(event `self.Box.OnComponentEndOverlap`
  (params (OverlappedComponent :type "PrimitiveComponent Object Reference") (OtherActor :type "Actor Object Reference") (OtherComp :type "PrimitiveComponent Object Reference") (OtherBodyIndex :type Integer))
  (if (== OtherActor (`self.Pawn`))
    (set `self.Pawn` null)
    (`self.OnPlayerEndOverlap` null)))

(fn `ReadyToImpact`
  (params (Player :type "Pawn Object Reference"))
  (returns (bReady :type Boolean))
  (return true))

(fn `UserConstructionScript`)