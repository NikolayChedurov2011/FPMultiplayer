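; BP_WeaponPickUp is a weapon pickup actor that adds a weapon to the inventory of an actor that touches it.
; On BeginPlay it takes its skeletal mesh from the class defaults of its WeaponClass.
; On box overlap it gets the other actor's inventory component through a message call.
; If that inventory lacks the weapon class, it adds it and destroys itself.
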(event `self.ReceiveBeginPlay`
  ;[1 1 1] В зависимости от класса оружия, устанавливаем нужный SkeletalMesh
  (`self.SetSkeletalMesh`))

(event `SetSkeletalMesh`
  (bind _weaponclass (`self.WeaponClass`))
  ;[1 1 1] В зависимости от класса оружия, устанавливаем нужный SkeletalMesh
  (if (`KismetSystemLibrary.IsValidClass` _weaponclass)
    (`SkinnedMeshComponent.SetSkinnedAssetAndUpdate` (`self.SkeletalMesh`) (`.SkeletalMeshObject` (defaults `Object` _weaponclass)) false)))

(event `self.Box.OnComponentBeginOverlap`
  (params (OverlappedComponent :type "PrimitiveComponent Object Reference") (OtherActor :type "Actor Object Reference") (OtherComp :type "PrimitiveComponent Object Reference") (OtherBodyIndex :type Integer) (bFromSweep :type Boolean) (SweepResult :type "HitResult Structure (by ref)"))
  ;[1 1 1] При оверлапе, проверяем, есть ли у нас уже этот класс оружия и если нет, то передаём класс оружия и добавляем его в инвентарь
  (bind _inventorycomponent (message `/Game/FPMultiplayer/Core/Interfaces/BPI_Inventory.GetInventoryComponent` OtherActor))
  (`/Engine/EditorBlueprintResources/StandardMacros.IsValid` _inventorycomponent
    (:`Is Valid`
      (if (not (`/Game/FPMultiplayer/Core/Characters/Components/BP_InventoryComponent.FindWeaponInArray` _inventorycomponent (`self.WeaponClass`)))
        (`/Game/FPMultiplayer/Core/Characters/Components/BP_InventoryComponent.AddWeapon` _inventorycomponent (`self.WeaponClass`))
        (`self.K2_DestroyActor`)))))

(fn `UserConstructionScript`)