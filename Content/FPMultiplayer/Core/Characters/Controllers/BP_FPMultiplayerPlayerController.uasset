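; Player controller for the first-person multiplayer mode that turns input into actions on the possessed BP_HumanoidPawn.
; Axis and action events drive movement, mouse look with a pawn rotation update on pitch, and jumping, while keys 1 and 2 request weapon slot equips through server events.
; Fire input sets a Firing flag, and Tick calls the pawn's ServerFireByWeapon every frame while it is held, giving continuous fire.
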(event `self.ReceiveBeginPlay`)

(event `self.ReceiveTick`
  (params (DeltaSeconds :type "Float (single-precision)"))
  ;[1 1 1] Если зажата клавиша стрельбы, то огонь будет вестись постоянно
  (`self.Try to Fire`))

(event `InputAxis|MoveForward`
  (params (AxisValue :type "Float (single-precision)"))
  (bind _returnvalue (`self.K2_GetPawn`))
  ;[1 0.2592 0.2393] Настройки управления
  ;;[1 1 1] Передвижение
  (bind _asbp_humanoid_pawn (cast `/Game/FPMultiplayer/Core/Characters/BasePawn/BP_HumanoidPawn` _returnvalue))
  (`Pawn.AddMovementInput` _asbp_humanoid_pawn (`self.GetActorForwardVector` _returnvalue) AxisValue false))

(event `InputAxis|MoveRight`
  (params (AxisValue :type "Float (single-precision)"))
  (bind _returnvalue (`self.K2_GetPawn`))
  ;[1 0.2592 0.2393] Настройки управления
  ;;[1 1 1] Передвижение
  (bind _asbp_humanoid_pawn (cast `/Game/FPMultiplayer/Core/Characters/BasePawn/BP_HumanoidPawn` _returnvalue))
  (`Pawn.AddMovementInput` _asbp_humanoid_pawn (`self.GetActorRightVector` _returnvalue) AxisValue false))

(event `InputAxis|MouseLookUp`
  (params (AxisValue :type "Float (single-precision)"))
  ;[1 0.2592 0.2393] Настройки управления
  ;;[1 1 1] Задаём управление камерой
  (`self.AddPitchInput` AxisValue)
  (bind _asbp_humanoid_pawn (cast `/Game/FPMultiplayer/Core/Characters/BasePawn/BP_HumanoidPawn` (`self.K2_GetPawn`)))
  (`/Game/FPMultiplayer/Core/Characters/BasePawn/BP_HumanoidPawn.Rot` _asbp_humanoid_pawn))

(event `InputAction|Jump`
  (params (Key :type "Key Structure"))
  ;[1 0.2592 0.2393] Настройки управления
  ;;[1 1 1] Прыжок
  (:`Pressed`
    (bind _asbp_humanoid_pawn (cast `/Game/FPMultiplayer/Core/Characters/BasePawn/BP_HumanoidPawn` (`self.K2_GetPawn`)))
    (`Character.Jump` _asbp_humanoid_pawn)))

(event `InputAxis|MouseLookHorizontal`
  (params (AxisValue :type "Float (single-precision)"))
  ;[1 0.2592 0.2393] Настройки управления
  ;;[1 1 1] Задаём управление камерой
  (`self.AddYawInput` AxisValue))

(event `Key|One`
  (params (Key :type "Key Structure"))
  ;[1 0.2592 0.2393] Настройки управления
  (:`Pressed`
    (bind _asbp_humanoid_pawn (cast `/Game/FPMultiplayer/Core/Characters/BasePawn/BP_HumanoidPawn` (`self.K2_GetPawn`)))
    (`/Game/FPMultiplayer/Core/Characters/BasePawn/BP_HumanoidPawn.Server_EquipSlot` _asbp_humanoid_pawn "NewEnumerator0")))

(event `InputAction|Fire`
  (params (Key :type "Key Structure"))
  ;[1 0.2592 0.2393] Настройки управления
  ;;[1 1 1] Стрельба
  (:`Pressed`
    (set `self.bFiring` true))
  (:`Released`
    (set `self.bFiring` false)))

(event `Key|Two`
  (params (Key :type "Key Structure"))
  ;[1 0.2592 0.2393] Настройки управления
  (:`Pressed`
    (bind _asbp_humanoid_pawn (cast `/Game/FPMultiplayer/Core/Characters/BasePawn/BP_HumanoidPawn` (`self.K2_GetPawn`)))
    (`/Game/FPMultiplayer/Core/Characters/BasePawn/BP_HumanoidPawn.Server_EquipSlot` _asbp_humanoid_pawn "NewEnumerator1")))

(fn `Try to Fire`
  ;[1 1 1] Вызываем событие стрельбы у персонажа
  (if (`self.bFiring`)
    (bind _asbp_humanoid_pawn (cast `/Game/FPMultiplayer/Core/Characters/BasePawn/BP_HumanoidPawn` (`self.K2_GetPawn`)))
    (`/Game/FPMultiplayer/Core/Characters/BasePawn/BP_HumanoidPawn.Server_FireByWeapon` _asbp_humanoid_pawn)))

(fn `UserConstructionScript`)