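; Inventory component for a humanoid pawn that stores its weapons by slot and tracks the one currently equipped.
; AddWeapon records the class, spawns the actor, hides the previous weapon, makes the new one current and attaches it to the owner's mesh at its bone.
; Multicast_EquipSlot switches between occupied slots by toggling visibility, then calls OnEquipped and binds the reload event.
; Helper functions return the current weapon and check whether a class is already held.
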(event `Multicast_EquipSlot`
  (params (Slot :type "/Game/FPMultiplayer/Core/Items/EWeaponSlot Enum" :default "NewEnumerator0"))
  (bind _currentweapon (`self.CurrentWeapon`))
  ;[1 1 1] Если у нас и у нового слота есть оружие и текущий слот не равен новому, то скрываем текущее оружие, а новое делаем текущим
  (if (and (`.ReturnValue` (`BlueprintMapLibrary.Map_Find` (`self.CurrentWeapons`) (`self.CurrentSlot`))) (`.ReturnValue` (`BlueprintMapLibrary.Map_Find` (`self.CurrentWeapons`) Slot)) (`|EnumInequality` Slot (`self.CurrentSlot`)))
    (`/Engine/EditorBlueprintResources/StandardMacros.IsValid` _currentweapon
      (:`Is Valid`
        (`Actor.SetActorHiddenInGame` _currentweapon true))
      (:`Is Not Valid`
        _))
    (bind _output_get (set `self.CurrentSlot` Slot))
    (bind _output_get_2 (set `self.CurrentWeapon` (`BlueprintMapLibrary.Map_Find` (`self.CurrentWeapons`) _output_get)))
    (`Actor.SetActorHiddenInGame` _output_get_2 false)
    (`/Game/FPMultiplayer/Core/Items/BP_BaseWeapon.OnEquipped` _output_get_2)
    (add `/Game/FPMultiplayer/Core/Items/BP_BaseWeapon.OnReload` (`self.CurrentWeapon`) (`|CreateDelegate` (cast `/Game/FPMultiplayer/Core/Characters/BasePawn/BP_HumanoidPawn` (`self.GetOwner`) :!pure true) :!event `OnReloadWeapon`))))

(fn `AddWeapon`
  (params (Weapon :type "/Game/FPMultiplayer/Core/Items/BP_BaseWeapon Class Reference"))
  (bind _returnvalue (`self.GetOwner`))
  (bind _currentweapon (`self.CurrentWeapon`))
  ;[1 1 1] Сохраняем ссылки на заспавненное оружие, атачим к персонажу и вызываем эвент у персонажа для локального атача оружия к рукам
  (`KismetArrayLibrary.Array_Add` (`self.Weapon`) Weapon)
  (`/Engine/EditorBlueprintResources/StandardMacros.IsValid` _currentweapon
    (:`Is Valid`
      (`Actor.SetActorHiddenInGame` _currentweapon true))
    (:`Is Not Valid`
      _))
  (bind _returnvalue_2 (`|SpawnActorFromClass` Weapon (`KismetMathLibrary.MakeTransform` (0.0 0.0 0.0)) "Undefined" "OverrideRootScale" null null))
  (bind _slot (`/Game/FPMultiplayer/Core/Items/BP_BaseWeapon.Slot` _returnvalue_2))
  (`BlueprintMapLibrary.Map_Add` (`self.CurrentWeapons`) _slot _returnvalue_2)
  (set `self.CurrentSlot` _slot)
  (bind _output_get (set `self.CurrentWeapon` _returnvalue_2))
  (`Actor.K2_AttachToComponent` _output_get (`/Game/FPMultiplayer/Core/Characters/BasePawn/BP_HumanoidPawn.GetMeshComponent` (cast `/Game/FPMultiplayer/Core/Characters/BasePawn/BP_HumanoidPawn` _returnvalue :!pure true)) (`/Game/FPMultiplayer/Core/Items/BP_BaseWeapon.AttachBone` _output_get) "KeepRelative" "KeepRelative" "KeepRelative" true)
  (`Actor.K2_SetActorRelativeTransform` _output_get (`/Game/FPMultiplayer/Core/Items/BP_BaseWeapon.TransformRelative` _output_get) false false)
  (`Actor.SetOwner` _output_get _returnvalue))

(fn `FindWeaponInArray`
  (params (WeaponClass :type "/Game/FPMultiplayer/Core/Items/BP_BaseWeapon Class Reference (by ref)"))
  (returns (ReturnValue :type Boolean))
  (return (not (== (`KismetArrayLibrary.Array_Find` (`self.Weapon`) WeaponClass) -1))))

(fn `GetCurrentWeapon`
  (returns (CurrentItem :type "/Game/FPMultiplayer/Core/Items/BP_BaseWeapon Object Reference"))
  (return (`self.CurrentWeapon`)))