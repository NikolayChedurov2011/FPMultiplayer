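; Health component for a BP_HumanoidPawn owner that tracks current health, damage, healing and death.
; On BeginPlay the server binds the owner's any-damage event to ApplyDamage, which clamps health at zero and sets Dead when it runs out.
; Damage and healing only apply while alive and broadcast OnHPChanged, while Dead's RepNotify broadcasts OnDeath.
; Tick prints current health on screen as debug output.
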(event `self.ReceiveBeginPlay`
  (bind _asbp_humanoid_pawn (cast `/Game/FPMultiplayer/Core/Characters/BasePawn/BP_HumanoidPawn` (`self.GetOwner`)))
  (bind _output_get (set `self.Owner` _asbp_humanoid_pawn))
  (if (`KismetSystemLibrary.IsServer`)
    (add `Actor.OnTakeAnyDamage` _output_get (delegate `ApplyAnyDamage`))))

(event `ApplyAnyDamage`
  (params (DamagedActor :type "Actor Object Reference") (Damage :type "Float (double-precision)") (DamageType :type "DamageType Object Reference") (InstigatedBy :type "Controller Object Reference") (DamageCauser :type "Actor Object Reference"))
  (`self.ApplyDamage` Damage))

(event `self.ReceiveTick`
  (params (DeltaSeconds :type "Float (single-precision)"))
  (`KismetSystemLibrary.PrintString` (`KismetStringLibrary.Concat_StrStr` "Health" (`KismetStringLibrary.Conv_DoubleToString` (`self.CurrentHealth`))) true true (struct :`G` 0.66 :`B` 1.0 :`A` 1.0) DeltaSeconds))

(fn `ApplyDamage`
  (params (Value :type "Float (double-precision)"))
  (if (`self.IsAlive`)
    (bind _output_get (set `self.CurrentHealth` (`KismetMathLibrary.FMax` (- (`self.CurrentHealth`) Value))))
    (`self.OnHPChanged` _output_get)
    (set `self.bDead` (== _output_get 0.0))))

(fn `ApplyHeal`
  (params (Value :type "Float (double-precision)"))
  (if (`self.IsAlive`)
    (bind _output_get (set `self.CurrentHealth` (`KismetMathLibrary.FMin` (+ Value (`self.CurrentHealth`)) (`self.MaxHealth`))))
    (`self.OnHPChanged` _output_get)))

(fn `IsAlive`
  (returns (ReturnValue :type Boolean))
  (return (> (`self.CurrentHealth`) 0.0)))

(fn `IsFull`
  (returns (ReturnValue :type Boolean))
  (return (== (`self.CurrentHealth`) (`self.MaxHealth`))))

(fn `OnRep_bDead`
  (if (`self.bDead`)
    (`self.OnDeath`)))