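; Multiplayer humanoid pawn with first-person arms for the local player and a body mesh for others.
; On possession the server creates rifle, pistol and knife in the inventory component, which handles switching and firing.
; It handles movement and look input, with multicast camera rotation sync for non-local copies.
; Death multicasts an animation flag, local unpossess with controller notification, and delayed destruction elsewhere, but its health-event binding never runs.
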(event `self.ReceivePossessed`
  (params (NewController :type "Controller Object Reference"))
  (bind _bp_inventorycomponent (`self.BP_InventoryComponent`))
  (`/Engine/EditorBlueprintResources/ActorMacros.Switch Has Authority`
    (:`Authority`
      (`/Game/FPMultiplayer/Core/Characters/Components/BP_InventoryComponent.CreateWeapon` _bp_inventorycomponent "/Game/FPMultiplayer/Items/AmmoWeapon/TraceWeapon/W_Rifle.W_Rifle_C")
      (`/Game/FPMultiplayer/Core/Characters/Components/BP_InventoryComponent.CreateWeapon` _bp_inventorycomponent "/Game/FPMultiplayer/Items/AmmoWeapon/TraceWeapon/W_Pistol.W_Pistol_C")
      (bind _createdweapon (`/Game/FPMultiplayer/Core/Characters/Components/BP_InventoryComponent.CreateWeapon` _bp_inventorycomponent "/Game/FPMultiplayer/Items/MeleeWeapon/W_Knife.W_Knife_C"))
      (set `/Game/FPMultiplayer/Core/Characters/Components/BP_InventoryComponent.CurrentWeapon` _createdweapon _bp_inventorycomponent))))

(event `self.ReceiveBeginPlay`)

(event `self.ReceiveTick`
  (params (DeltaSeconds :type "Float (single-precision)"))
  (set `self.bArmed` (`KismetSystemLibrary.IsValid` (`/Game/FPMultiplayer/Core/Characters/Components/BP_InventoryComponent.GetCurrentWeapon` (`self.BP_InventoryComponent`)))))

(event `Client_Reload`
  ;[1 1 1] Смена оружия и перезарядка
  (cast `/Game/FPMultiplayer/Core/Items/AmmoWeapon/BP_AmmoWeapon` (`/Game/FPMultiplayer/Core/Characters/Components/BP_InventoryComponent.GetCurrentWeapon` (`self.BP_InventoryComponent`)))
  (`self.Server_Reload`))

(event `ChangeWeapon`
  (params (Slot :type "/Game/FPMultiplayer/Core/Items/EweaponType Enum" :default "NewEnumerator0"))
  ;[1 1 1] Смена оружия и перезарядка
  (`/Game/FPMultiplayer/Core/Characters/Components/BP_InventoryComponent.ChangeWeaponFromClient` (`self.BP_InventoryComponent`) Slot))

(event `Server_FireByWeapon`
  (params (bActivate :type Boolean))
  (bind _currentitem (`/Game/FPMultiplayer/Core/Characters/Components/BP_InventoryComponent.GetCurrentWeapon` (`self.BP_InventoryComponent`)))
  ;[1 1 1] Стрельба из оружия
  (if bActivate
    (`/Game/FPMultiplayer/Core/Items/BP_BaseWeapon.Fire` _currentitem)
    (else
      (`/Game/FPMultiplayer/Core/Items/BP_BaseWeapon.StopUseWeapon` _currentitem))))

(event `Server_Reload`
  ;[1 1 1] Смена оружия и перезарядка
  (bind _asbp_ammo_weapon (cast `/Game/FPMultiplayer/Core/Items/AmmoWeapon/BP_AmmoWeapon` (`/Game/FPMultiplayer/Core/Characters/Components/BP_InventoryComponent.GetCurrentWeapon` (`self.BP_InventoryComponent`))))
  (set `/Game/FPMultiplayer/Core/Items/AmmoWeapon/BP_AmmoWeapon.bReloading` true _asbp_ammo_weapon))

(event `ScrollWeapon`
  (params (bNextWeapon :type Boolean))
  ;[1 1 1] Смена оружия и перезарядка
  (`/Game/FPMultiplayer/Core/Characters/Components/BP_InventoryComponent.ScrollWeaponFromClient` (`self.BP_InventoryComponent`) bNextWeapon))

(event `Rot`
  ;[1 1 1] Синхронизируем поворот персонажа с сервером
  (if (not (`self.IsLocallyControlled`))
    (`self.Multicast_SyncRotation` (`self.GetControlRotation`))))

(event `MoveForward`
  (params (ScaleValue :type "Float (double-precision)"))
  ;[1 1 1] Управление персонажем
  (`self.AddMovementInput` (`self.GetActorForwardVector`) ScaleValue))

(event `InputAxis|MouseLookUp`
  (params (AxisValue :type "Float (single-precision)"))
  ;[1 1 1] Управление персонажем
  (`self.AddControllerPitchInput` AxisValue)
  (`self.Rot`))

(event `InputAxis|MouseLookHorizontal`
  (params (AxisValue :type "Float (single-precision)"))
  ;[1 1 1] Управление персонажем
  (`self.AddControllerYawInput` AxisValue))

(event `Multicast_SyncRotation`
  (params (SyncRotation :type "Rotator Structure"))
  ;[1 1 1] Синхронизируем поворот персонажа с сервером
  (set `self.SyncRotation` SyncRotation)
  (if (not (`self.IsLocallyControlled`))
    (`SceneComponent.K2_SetWorldRotation` (`self.Camera`) (`self.SyncRotation`) false false)))

(event `MoveRight`
  (params (ScaleValue :type "Float (double-precision)"))
  ;[1 1 1] Управление персонажем
  (`self.AddMovementInput` (`self.GetActorRightVector`) ScaleValue))

(event `ToJump`
  ;[1 1 1] Управление персонажем
  (`self.Jump`))

(event `Server_OnDeath`
  ;[1 1 1] Событие смерти
  (`/Engine/EditorBlueprintResources/ActorMacros.Switch Has Authority`
    (:`Authority`
      (`self.Multicast_OnDeath`))))

(event `Multicast_OnDeath`
  (bind _returnvalue (`GameplayStatics.GetPlayerController` 0))
  ;[1 1 1] Событие смерти
  (set `/Game/FPMultiplayer/Characters/TestCharacter/ABP_TestCharacter_ThirdPerson.bDead` true (cast `/Game/FPMultiplayer/Characters/TestCharacter/ABP_TestCharacter_ThirdPerson` (`SkeletalMeshComponent.GetAnimInstance` (`self.Mesh`)) :!pure true))
  (if (`self.IsLocallyControlled`)
    (`Controller.UnPossess` _returnvalue)
    (`/Game/FPMultiplayer/Core/Characters/Controllers/BP_FPMultiplayerPlayerController.Server_OnCharacterDead` (cast `/Game/FPMultiplayer/Core/Characters/Controllers/BP_FPMultiplayerPlayerController` _returnvalue :!pure true) (`self.GetTransform`))
    (else
      (`KismetSystemLibrary.Delay` 7.0)
      (`self.K2_DestroyActor`))))

(fn `GetHealthComponent`
  (returns (HealthComponent :type "/Game/FPMultiplayer/Core/Characters/Components/BP_HealthComponent Object Reference"))
  (return (`self.BP_HealthComponent`)))

(fn `GetInventoryComponent`
  (returns (InventoryComponent :type "/Game/FPMultiplayer/Core/Characters/Components/BP_InventoryComponent Object Reference"))
  (return (`self.BP_InventoryComponent`)))

(fn `GetMeshComponent`
  (returns (SkeletalMesh :type "SkeletalMeshComponent Object Reference"))
  (return (select `bool` (`self.IsLocallyControlled`) :`false` (`self.Mesh`) :`true` (`self.CharacterMesh_Arms`))))

(fn `GetPawn`
  (returns (Pawn :type "Pawn Object Reference"))
  (return self))

(fn `GetSyncRotation`
  (returns (SyncRotation :type "Rotator Structure"))
  (return (`self.SyncRotation`)))

(fn `UserConstructionScript`)