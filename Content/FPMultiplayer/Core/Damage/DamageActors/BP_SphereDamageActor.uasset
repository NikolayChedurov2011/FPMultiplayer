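; BP_SphereDamageActor is the spherical variant of a damage actor, supplying the shape query that finds actors within a radius.
; ShapeOverlapObject runs a sphere overlap at the actor's location using SphereRadius and the given object types, then returns the overlapped actors.
; An optional debug flag draws the sphere briefly.
; The event graph is inactive and the construction script only calls the parent, so this file applies no damage itself.
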(fn `ShapeOverlapObject`
  (params (ObjectTypes :type "Array of EObjectTypeQuery Enum (by ref)" :default _))
  (returns (OverlapedActors :type "Array of Actor Object Reference"))
  (bind _returnvalue (`self.K2_GetActorLocation`))
  (bind _sphereradius (`self.SphereRadius`))
  (bind _outactors (`KismetSystemLibrary.SphereOverlapActors` _returnvalue _sphereradius ObjectTypes))
  (if (`self.bDrawFebug`)
    (`KismetSystemLibrary.DrawDebugSphere` _returnvalue _sphereradius 12 (struct :`R` 1.0 :`G` 1.0 :`B` 1.0 :`A` 1.0) 1.0 1.0))
  (return _outactors))

(fn `UserConstructionScript`
  (`parent.UserConstructionScript`))