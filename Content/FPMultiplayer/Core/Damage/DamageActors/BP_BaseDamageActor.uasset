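; BP_BaseDamageActor is a base actor that deals one-shot damage to overlapped actors, then destroys itself.
; BeginPlay calls a server damage event, which queries ShapeOverlapObject with the configured object types and passes the result to OnOverlapedActors.
; That handler applies DamageValue to each actor, with itself as damage causer, before destroying itself.
; ShapeOverlapObject is an empty stub here, so this class alone supplies no overlap shape.
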(event `self.ReceiveBeginPlay`
  (`self.Server_DamageBegin`))

(event `Server_DamageBegin`
  (bind _overlapedactors (`self.ShapeOverlapObject` (`self.OverlapObjectTypes`)))
  (`self.OnOverlapedActors` _overlapedactors))

(fn `ApplyDamageForActors`
  (params (InActors :type "Array of Actor Object Reference"))
  (for _array_element InActors
    (`GameplayStatics.ApplyDamage` _array_element (`self.DamageValue`) null self))
  (return))

(fn `OnOverlapedActors`
  (params (OverlapedActors :type "Array of Actor Object Reference"))
  (`self.ApplyDamageForActors` OverlapedActors)
  (`self.K2_DestroyActor`))

(fn `ShapeOverlapObject`
  (params (ObjectTypes :type "Array of EObjectTypeQuery Enum"))
  (returns (OverlapedActors :type "Array of Actor Object Reference"))
  (return))

(fn `UserConstructionScript`)