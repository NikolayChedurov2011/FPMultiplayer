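; Med kit pickup for the FPMultiplayer game, apparently an unfinished child of a rechargeable pickup base.
; It overrides PlayerImpact and ReadyToImpact, calling the parent and fetching the player's health component through a GetHealthComponentMessage call.
; The validity branches are empty, so no healing happens here.
; ReadyToImpact combines the parent result and component validity with a constant false, so it always returns false.
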(event `self.PlayerImpact`
  (params (Player :type "Pawn Object Reference"))
  (`parent.PlayerImpact` Player)
  (bind _healthcomponent (message `/Game/FPMultiplayer/Core/Interfaces/BPI_Health.GetHealthComponent` Player))
  (`/Engine/EditorBlueprintResources/StandardMacros.IsValid` _healthcomponent))

(fn `ReadyToImpact`
  (params (Player :type "Pawn Object Reference"))
  (returns (bReady :type Boolean))
  (bind _bready (`parent.ReadyToImpact` Player))
  (bind _healthcomponent (message `/Game/FPMultiplayer/Core/Interfaces/BPI_Health.GetHealthComponent` Player))
  (`/Engine/EditorBlueprintResources/StandardMacros.IsValid` _healthcomponent
    (:`Is Valid`
      _)
    (:`Is Not Valid`
      _))
  (return (and (`KismetSystemLibrary.IsValid` _healthcomponent) _bready false)))

(fn `UserConstructionScript`
  (`parent.UserConstructionScript`))