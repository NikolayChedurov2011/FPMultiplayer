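; BP_Ammo is a rechargeable pickup that gives ammo to the player's currently equipped weapon.
; ReadyToImpact adds to the parent check that the player is alive and holds a BP_AmmoWeapon that is not full.
; On PlayerImpact it runs the parent logic, then applies AmmoValue to that weapon.
; Player components are fetched through GetInventoryComponentMessage and GetHealthComponentMessage calls rather than casting the player.
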(event `/Game/FPMultiplayer/Core/PickUps/BP_BasePickUp.PlayerImpact`
  (params (Player :type "Pawn Object Reference"))
  (`parent.PlayerImpact` Player)
  (bind _inventorycomponent (message `/Game/FPMultiplayer/Core/Interfaces/BPI_Inventory.GetInventoryComponent` Player))
  (`/Engine/EditorBlueprintResources/StandardMacros.IsValid` _inventorycomponent
    (:`Is Valid`
      (bind _currentweapon (`/Game/FPMultiplayer/Core/Characters/Components/BP_InventoryComponent.CurrentWeapon` _inventorycomponent))
      (`/Engine/EditorBlueprintResources/StandardMacros.IsValid` _currentweapon
        (:`Is Valid`
          (`/Game/FPMultiplayer/Core/Items/AmmoWeapon/BP_AmmoWeapon.ApplyAmmo` (cast `/Game/FPMultiplayer/Core/Items/AmmoWeapon/BP_AmmoWeapon` _currentweapon :!pure true) (`self.AmmoValue`)))))))

(fn `ReadyToImpact`
  (params (Player :type "Pawn Object Reference"))
  (returns (bReady :type Boolean))
  (bind _bready (`parent.ReadyToImpact` Player))
  (bind _healthcomponent (message `/Game/FPMultiplayer/Core/Interfaces/BPI_Health.GetHealthComponent` Player))
  (`/Engine/EditorBlueprintResources/StandardMacros.IsValid` _healthcomponent
    (:`Is Valid`
      (bind _inventorycomponent (message `/Game/FPMultiplayer/Core/Interfaces/BPI_Inventory.GetInventoryComponent` Player))
      (`/Engine/EditorBlueprintResources/StandardMacros.IsValid` _inventorycomponent
        (:`Is Valid`
          (bind _currentweapon (`/Game/FPMultiplayer/Core/Characters/Components/BP_InventoryComponent.CurrentWeapon` _inventorycomponent))
          (`/Engine/EditorBlueprintResources/StandardMacros.IsValid` _currentweapon
            (:`Is Valid`
              (bind _asbp_ammo_weapon (cast `/Game/FPMultiplayer/Core/Items/AmmoWeapon/BP_AmmoWeapon` _currentweapon))
              (return (and (not (`/Game/FPMultiplayer/Core/Items/AmmoWeapon/BP_AmmoWeapon.IsFullAmmo` _asbp_ammo_weapon)) _bready (`/Game/FPMultiplayer/Core/Characters/Components/BP_HealthComponent.IsAlive` _healthcomponent))))))))))

(fn `UserConstructionScript`
  (`parent.UserConstructionScript`))