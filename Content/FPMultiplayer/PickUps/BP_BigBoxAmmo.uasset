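; BP_BigBoxAmmo is an ammo box pickup that refills the player's current weapon.
; ReadyToImpact allows pickup only if the parent check passes, the player is alive and the held weapon is a BP_AmmoWeapon that is not full.
; PlayerImpact runs the parent behavior, then applies AmmoValue to that weapon.
; Both reach the inventory component through message calls on the player, and the readiness check gets health the same way.
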(event `self.PlayerImpact`
  (params (Player :type "Pawn Object Reference"))
  (`parent.PlayerImpact` Player)
  (bind _inventorycomponent (message `/Game/FPMultiplayer/Core/Interfaces/BPI_Inventory.GetInventoryComponent` Player))
  (`/Engine/EditorBlueprintResources/StandardMacros.IsValid` _inventorycomponent
    (:`Is Valid`
      (bind _currentitem (`/Game/FPMultiplayer/Core/Characters/Components/BP_InventoryComponent.GetCurrentWeapon` _inventorycomponent))
      (`/Engine/EditorBlueprintResources/StandardMacros.IsValid` _currentitem
        (:`Is Valid`
          (`/Game/FPMultiplayer/Core/Items/AmmoWeapon/BP_AmmoWeapon.ApplyAmmo` (cast `/Game/FPMultiplayer/Core/Items/AmmoWeapon/BP_AmmoWeapon` _currentitem :!pure true) (`self.AmmoValue`)))))))

(fn `ReadyToImpact`
  (params (Player :type "Pawn Object Reference"))
  (returns (bReady :type Boolean))
  (bind _bready (`parent.ReadyToImpact` Player))
  (bind _healthcomponent (message `/Game/FPMultiplayer/Core/Interfaces/BPI_Health.GetHealthComponent` Player))
  (bind _inventorycomponent (message `/Game/FPMultiplayer/Core/Interfaces/BPI_Inventory.GetInventoryComponent` Player))
  (`/Engine/EditorBlueprintResources/StandardMacros.IsValid` _inventorycomponent
    (:`Is Valid`
      (bind _currentitem (`/Game/FPMultiplayer/Core/Characters/Components/BP_InventoryComponent.GetCurrentWeapon` _inventorycomponent))
      (`/Engine/EditorBlueprintResources/StandardMacros.IsValid` _currentitem
        (:`Is Valid`
          (bind _asbp_ammo_weapon (cast `/Game/FPMultiplayer/Core/Items/AmmoWeapon/BP_AmmoWeapon` _currentitem :!pure true))
          (`/Engine/EditorBlueprintResources/StandardMacros.IsValid` _asbp_ammo_weapon
            (:`Is Valid`
              (return (and (not (`/Game/FPMultiplayer/Core/Items/AmmoWeapon/BP_AmmoWeapon.IsFullAmmo` _asbp_ammo_weapon)) _bready (`/Game/FPMultiplayer/Core/Characters/Components/BP_HealthComponent.IsAlive` _healthcomponent))))))))))

(fn `UserConstructionScript`
  (`parent.UserConstructionScript`))